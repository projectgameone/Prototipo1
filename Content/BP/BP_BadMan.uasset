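; BP_BadMan is a 2D sprite enemy that chases and shoots the player and drops a random item on death.
; Each Tick it yaws toward the player, steps along X when within range, and fires if the signed X distance is below a threshold.
; A DoOnce with Delay limits BP_BadManBullet spawns from its Arrow to roughly one per second.
; DMGBadMan subtracts health, printing the remainder or destroying the actor.
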(event Custom|DMGBadMan
  (params (DmgTaken :type Integer))
  ;[1 1 1] Sistema Danni BadMan
  (bind _output_get (Variables|Default|SetBadMan_Health (- (Variables|Default|GetBadMan_Health) DmgTaken)))
  (if (<= _output_get 0)
    (Actor|DestroyActor)
    ;[1 1 1] Rilascio Oggetti
    (Game|SpawnActorfromClass (Utilities|Array|Get(acopy) (Variables|Default|GetItemDrop) (Math|Random|RandomIntegerinRange 0 2)) (Math|Conversions|ToTransform(Vector) (Transformation|GetActorLocation)) "Undefined" 0 0)
    (else
      (Development|PrintString (Utilities|String|ToString(Integer) (Variables|Default|GetBadMan_Health))))))

(event Custom|BadManShot
  ;[1 1 1] BadMan Spara
  (Utilities|FlowControl|DoOnce false :!label _label
    (:Completed
      (Utilities|FlowControl|Sequence
        (:then_0
          (Audio|PlaySoundatLocation "/Game/Sounds/shot_Cue.shot_Cue" "0, 0, 0"))
        (:then_1
          (Game|SpawnActorfromClass "/Game/BP/BP_BadManBullet.BP_BadManBullet_C" (Transformation|GetWorldTransform (Variables|Default|GetArrow)) "Undefined" 0 0)
          (Utilities|FlowControl|Delay 1.0)
          (goto _label Reset))))))

(event EventBeginPlay)

(event EventActorBeginOverlap
  (params (OtherActor :type Actor%20Object%20Reference)))

(event EventTick
  (params (DeltaSeconds :type Float%20%28single-precision%29))
  (bind _returnvalue (Transformation|GetActorLocation))
  ;[1 1 1] BadMan Movimento
  (Utilities|FlowControl|Sequence
    (:then_0
      (bind _output_get (Variables|Default|SetDistance (- (.x (Transformation|GetWorldLocation (Variables|Default|GetPaperSprite))) (.x (Transformation|GetActorLocation (Game|GetPlayerCharacter 0))))))
      (if (<= _output_get 977.0)
        (CallFunction|BadManShot)))
    (:then_1
      (Transformation|SetActorRotation (Math|Rotator|MakeRotator 0.0 0.0 (.yaw (Math|Rotator|FindLookatRotation (Transformation|GetActorLocation) (Transformation|GetActorLocation (Game|GetPlayerCharacter 0)))))))
    (:then_2
      (Variables|Default|SetActorX (.x _returnvalue)))
    (:then_3
      (Variables|Default|SetActorY (.y _returnvalue)))
    (:then_4
      (Variables|Default|SetActorZ (.z _returnvalue)))
    (:then_5
      (if (Math|Float|InRange(Float) (Variables|Default|GetDistance) 0.0 7e+02)
        (Transformation|SetActorLocation (Math|Vector|MakeVector (- (Variables|Default|GetActorX) 5.0) (Variables|Default|GetActorY) (Variables|Default|GetActorZ)) false false)))
    (:then_6
      (if (Math|Float|InRange(Float) (Variables|Default|GetDistance) -7e+02 0.0)
        (Transformation|SetActorLocation (Math|Vector|MakeVector (+ (Variables|Default|GetActorX) 5.0) (Variables|Default|GetActorY) (Variables|Default|GetActorZ)) false false)))))

(fn ConstructionScript)