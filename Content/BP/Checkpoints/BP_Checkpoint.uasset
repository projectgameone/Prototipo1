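; Checkpoint actor for the 2D side-scroller that saves progress to slot "Loc" when an actor tagged "Tommy" overlaps it.
; It fills a new Save_Info object with player location and level, saving once via DoOnce.
; The CheckPoint flag selects whether health, bullets, coins and lives are copied before saving or only afterwards, leaving them unwritten.
; The construction script sizes the trigger box and picks the billboard sprite from that flag.
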(event Collision|EventActorBeginOverlap
  (params (OtherActor :type Actor%20Object%20Reference))
  (if (Actor|ActorHasTag OtherActor "Tommy")
    (bind _returnvalue (SaveGame|CreateSaveGameObject "/Game/BP/Checkpoints/Save_Info.Save_Info_C"))
    (bind _assave_info (Utilities|Casting|CastToSave_Info _returnvalue))
    (Variables|Default|SetSaveInfo _assave_info)
    (bind _as2dside_scroller_character (Utilities|Casting|CastTo2DSideScrollerCharacter (Game|GetPlayerCharacter 0)))
    (Variables|Default|SetCharInfo _as2dside_scroller_character)
    (if (Variables|Default|GetCheckPoint)
      (Utilities|FlowControl|DoOnce false
        (:Completed
          (Variables|/Game/BP/Checkpoints/Save_Info.Save_Info_C|SetCheckLocation (Variables|Default|GetSaveInfo) (Math|Vector|MakeVector (.x (Transformation|GetActorLocation (Variables|Default|GetCharInfo))) (.y (Transformation|GetActorLocation (Variables|Default|GetCharInfo))) (.z (Transformation|GetActorLocation (Variables|Default|GetCharInfo)))))
          (bind _returnvalue_2 (Game|GetCurrentLevelName true))
          (Variables|/Game/BP/Checkpoints/Save_Info.Save_Info_C|SetCurrentLevel (Variables|Default|GetSaveInfo) (Utilities|String|StringToName _returnvalue_2))
          (Utilities|FlowControl|Sequence
            (:then_0
              (Variables|/Game/BP/Checkpoints/Save_Info.Save_Info_C|SetSavedHealth (Variables|Default|GetSaveInfo) (Variables|/Game/2DSideScrollerBP/Blueprints/2DSideScrollerCharacter.2DSideScrollerCharacter_C|GetCharHealth (Variables|Default|GetCharInfo))))
            (:then_1
              (Variables|/Game/BP/Checkpoints/Save_Info.Save_Info_C|SetSavedBullets (Variables|Default|GetSaveInfo) (Variables|/Game/2DSideScrollerBP/Blueprints/2DSideScrollerCharacter.2DSideScrollerCharacter_C|GetCurrentBullets (Variables|Default|GetCharInfo))))
            (:then_2
              (Variables|/Game/BP/Checkpoints/Save_Info.Save_Info_C|SetSavedCoin (Variables|Default|GetSaveInfo) (Variables|/Game/2DSideScrollerBP/Blueprints/2DSideScrollerCharacter.2DSideScrollerCharacter_C|GetCharCoins (Variables|Default|GetCharInfo))))
            (:then_3
              (Variables|/Game/BP/Checkpoints/Save_Info.Save_Info_C|SetSavedLives (Variables|Default|GetSaveInfo) (Variables|/Game/2DSideScrollerBP/Blueprints/2DSideScrollerCharacter.2DSideScrollerCharacter_C|GetCharLives (Variables|Default|GetCharInfo))))
            (:then_4
              (SaveGame|SaveGametoSlot (Variables|Default|GetSaveInfo) "Loc")
              (Development|PrintString (Utilities|String|ToString(Name) (stale _output_get)) :!label _label)))))
      (else
        (Utilities|FlowControl|DoOnce false
          (:Completed
            (Variables|/Game/BP/Checkpoints/Save_Info.Save_Info_C|SetCheckLocation (Variables|Default|GetSaveInfo) (Math|Vector|MakeVector (.x (Transformation|GetActorLocation (Variables|Default|GetCharInfo))) (.y (Transformation|GetActorLocation (Variables|Default|GetCharInfo))) (.z (Transformation|GetActorLocation (Variables|Default|GetCharInfo)))))
            (bind _returnvalue_3 (Game|GetCurrentLevelName true))
            (bind _output_get (Variables|/Game/BP/Checkpoints/Save_Info.Save_Info_C|SetCurrentLevel (Variables|Default|GetSaveInfo) (Utilities|String|StringToName _returnvalue_3)))
            (Utilities|FlowControl|Sequence
              (:then_0
                (SaveGame|SaveGametoSlot (Variables|Default|GetSaveInfo) "Loc")
                (goto _label))
              (:then_1
                (Variables|/Game/BP/Checkpoints/Save_Info.Save_Info_C|SetSavedBullets (Variables|Default|GetSaveInfo) (Variables|/Game/2DSideScrollerBP/Blueprints/2DSideScrollerCharacter.2DSideScrollerCharacter_C|GetCurrentBullets (Variables|Default|GetCharInfo))))
              (:then_2
                (Variables|/Game/BP/Checkpoints/Save_Info.Save_Info_C|SetSavedCoin (Variables|Default|GetSaveInfo) (Variables|/Game/2DSideScrollerBP/Blueprints/2DSideScrollerCharacter.2DSideScrollerCharacter_C|GetCharCoins (Variables|Default|GetCharInfo))))
              (:then_3
                (Variables|/Game/BP/Checkpoints/Save_Info.Save_Info_C|SetSavedLives (Variables|Default|GetSaveInfo) (Variables|/Game/2DSideScrollerBP/Blueprints/2DSideScrollerCharacter.2DSideScrollerCharacter_C|GetCharLives (Variables|Default|GetCharInfo))))
              (:then_4
                (Variables|/Game/BP/Checkpoints/Save_Info.Save_Info_C|SetSavedHealth (Variables|Default|GetSaveInfo) (Variables|/Game/2DSideScrollerBP/Blueprints/2DSideScrollerCharacter.2DSideScrollerCharacter_C|GetCharHealth (Variables|Default|GetCharInfo)))))))))))

(fn ConstructionScript
  (Components|Box|SetBoxExtent (Variables|Default|GetBox) (Variables|Default|GetChangeHitBox) true)
  (if (Variables|Default|GetCheckPoint)
    (Rendering|Components|Sprite|SetSprite (Variables|Default|GetBillboard) "/Game/BP/Checkpoints/C.C")
    (else
      (Rendering|Components|Sprite|SetSprite (Variables|Default|GetBillboard) "/Game/BP/Checkpoints/S.S"))))